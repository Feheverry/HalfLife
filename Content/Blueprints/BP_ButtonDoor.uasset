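; Button-door actor that shows an interaction prompt widget while the first-person character stands in its Box trigger; no door movement is implemented.
; Overlap begin adds the UI_PlayerInteract widget and opens a Gate, and overlap end removes the widget and closes it.
; The Gate's exit spawns an impact Niagara effect at the Niagara component, but nothing shown enters the Gate.
; BeginPlay enables player input, though no input event is present.
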(event OnComponentBeginOverlap(Box)
  (params (OverlappedComponent :type Primitive%20Component%20Object%20Reference) (OtherActor :type Actor%20Object%20Reference) (OtherComp :type Primitive%20Component%20Object%20Reference) (OtherBodyIndex :type Integer) (bFromSweep :type Boolean) (SweepResult :type Hit%20Result%20Structure%20%28by%20ref%29))
  (Utilities|Casting|CastToFirstPersonCharacter OtherActor)
  (bind _returnvalue (UserInterface|CreateWidget "/Game/Blueprints/UI_PlayerInteract.UI_PlayerInteract_C"))
  (UserInterface|Viewport|AddtoViewport _returnvalue 0)
  (Utilities|FlowControl|Gate false ; enters at Open
    (:Exit
      (Niagara|SpawnSystematLocation "/Game/sA_Megapack_v1/sA_ShootingVfxPack/FX/NiagaraSystems/NS_Impact_1.NS_Impact_1" (Transformation|GetWorldLocation (Variables|Default|GetNiagara))))))

(event OnComponentEndOverlap(Box)
  (params (OverlappedComponent :type Primitive%20Component%20Object%20Reference) (OtherActor :type Actor%20Object%20Reference) (OtherComp :type Primitive%20Component%20Object%20Reference) (OtherBodyIndex :type Integer))
  (Utilities|Casting|CastToFirstPersonCharacter OtherActor)
  (Widget|RemovefromParent (stale OnComponentBeginOverlap(Box) _returnvalue))
  (Utilities|FlowControl|Gate false ; enters at Close
    (:Exit
      (Niagara|SpawnSystematLocation "/Game/sA_Megapack_v1/sA_ShootingVfxPack/FX/NiagaraSystems/NS_Impact_1.NS_Impact_1" (Transformation|GetWorldLocation (Variables|Default|GetNiagara))))))

(event EventBeginPlay
  (Input|EnableInput (Game|GetPlayerController 0)))

(event Collision|EventActorBeginOverlap
  (params (OtherActor :type Actor%20Object%20Reference)))

(event EventTick
  (params (DeltaSeconds :type Float%20%28single-precision%29)))

(fn ConstructionScript)