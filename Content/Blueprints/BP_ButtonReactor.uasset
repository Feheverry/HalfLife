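; BP_ButtonReactor is an interactable reactor button that triggers an explosion and ends the game.
; Overlapping its box with the FirstPersonCharacter shows a warning widget and opens a gate for the Interact input, which is enabled at BeginPlay; leaving removes the widget and closes it.
; Interacting while in range spawns a Niagara explosion, then after a short delay shows the game-over UI, pauses the game and shows the cursor.
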(event OnComponentBeginOverlap(Box)
  (params (OverlappedComponent :type Primitive%20Component%20Object%20Reference) (OtherActor :type Actor%20Object%20Reference) (OtherComp :type Primitive%20Component%20Object%20Reference) (OtherBodyIndex :type Integer) (bFromSweep :type Boolean) (SweepResult :type Hit%20Result%20Structure%20%28by%20ref%29))
  (Utilities|Casting|CastToFirstPersonCharacter OtherActor)
  (bind _returnvalue (UserInterface|CreateWidget "/Game/Blueprints/UI_PlayerWarning.UI_PlayerWarning_C"))
  (UserInterface|Viewport|AddtoViewport _returnvalue 0)
  (Utilities|FlowControl|Gate true) ; enters at Open
)

(event OnComponentEndOverlap(Box)
  (params (OverlappedComponent :type Primitive%20Component%20Object%20Reference) (OtherActor :type Actor%20Object%20Reference) (OtherComp :type Primitive%20Component%20Object%20Reference) (OtherBodyIndex :type Integer))
  (Utilities|Casting|CastToFirstPersonCharacter OtherActor)
  (Widget|RemovefromParent (stale OnComponentBeginOverlap(Box) _returnvalue))
  (Utilities|FlowControl|Gate true) ; enters at Close
)

(event EventBeginPlay
  (Input|EnableInput (Game|GetPlayerController 0)))

(event Collision|EventActorBeginOverlap
  (params (OtherActor :type Actor%20Object%20Reference)))

(event EventTick
  (params (DeltaSeconds :type Float%20%28single-precision%29)))

(event Input|ActionEvents|InputActionInteract
  (params (Key :type Key%20Structure :default "None"))
  (:Pressed
    (Utilities|FlowControl|Gate true
      (:Exit
        (Niagara|SpawnSystematLocation "/Game/sA_Megapack_v1/sA_ShootingVfxPack/FX/NiagaraSystems/NS_Explossion.NS_Explossion" (Transformation|GetWorldLocation (Variables|Default|GetNiagara)))
        (Utilities|FlowControl|Delay 0.5)
        (bind _returnvalue (UserInterface|CreateWidget "/Game/Blueprints/UI_GameOver.UI_GameOver_C"))
        (UserInterface|Viewport|AddtoViewport _returnvalue 0)
        (Game|SetGamePaused true)
        (Variables|/Script/Engine.PlayerController|SetbShowMouseCursor (Game|GetPlayerController 0) true)))))

(fn ConstructionScript)