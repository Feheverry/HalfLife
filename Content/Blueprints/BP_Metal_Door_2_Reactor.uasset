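; Two-panel sliding metal door that opens when anything overlaps its Box trigger, named for the reactor area.
; After a three-second delay, two timelines play to drive the relative Y location of the Left and Right components separately.
; Ending the overlap stops both timelines after the same delay rather than reversing them, so the Blueprint has no closing logic.
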(event OnComponentBeginOverlap(Box)
  (params (OverlappedComponent :type Primitive%20Component%20Object%20Reference) (OtherActor :type Actor%20Object%20Reference) (OtherComp :type Primitive%20Component%20Object%20Reference) (OtherBodyIndex :type Integer) (bFromSweep :type Boolean) (SweepResult :type Hit%20Result%20Structure%20%28by%20ref%29))
  ;[1 1 1] Left Door
  (Utilities|FlowControl|Delay 3.0)
  (Utilities|FlowControl|Sequence
    (:then_0
      (bind _left (Timeline|Timeline_0 Play)
        (:Update
          (Transformation|SetRelativeLocation (Variables|Default|GetLeft) (Math|Vector|MakeVector 0.0 _left 0.0) false false))))
    (:then_1
      ;[1 1 1] Right Door
      (bind _right (Timeline|Timeline_1 Play)
        (:Update
          (Transformation|SetRelativeLocation (Variables|Default|GetRight) (Math|Vector|MakeVector 0.0 _right 0.0) false false))))))

(event OnComponentEndOverlap(Box)
  (params (OverlappedComponent :type Primitive%20Component%20Object%20Reference) (OtherActor :type Actor%20Object%20Reference) (OtherComp :type Primitive%20Component%20Object%20Reference) (OtherBodyIndex :type Integer))
  ;[1 1 1] Right Door
  (Utilities|FlowControl|Delay 3.0)
  (Utilities|FlowControl|Sequence
    (:then_0
      ;[1 1 1] Left Door
      (bind _left (Timeline|Timeline_0 Stop)
        (:Update
          (Transformation|SetRelativeLocation (Variables|Default|GetLeft) (Math|Vector|MakeVector 0.0 _left 0.0) false false))))
    (:then_1
      (bind _right (Timeline|Timeline_1 Stop)
        (:Update
          (Transformation|SetRelativeLocation (Variables|Default|GetRight) (Math|Vector|MakeVector 0.0 _right 0.0) false false))))))

(fn ConstructionScript)